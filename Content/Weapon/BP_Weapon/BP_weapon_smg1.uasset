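; SMG weapon Blueprint that currently holds only a hit-scan impact sound test bound to the Q key.
; Pressing Q runs a debug-drawn line trace forward from the first-person camera of the referenced NewVar object.
; The hit's physical material surface type selects a sound to play at the impact point, with only concrete assigned so far.
; It contains no damage or ammo logic, and construction is empty.
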(event `Key|Q`
  (params (Key :type "Key Structure"))
  (bind _firstpersoncamera (`MyCharacter.FirstPersonCamera` (`self.NewVar`)))
  (bind _returnvalue (`SceneComponent.K2_GetComponentLocation` _firstpersoncamera))
  (:`Pressed`
    (bind _outhit (`KismetSystemLibrary.LineTraceSingle` :`Start` _returnvalue :`End` (+ _returnvalue (* (`SceneComponent.GetForwardVector` _firstpersoncamera) (`KismetMathLibrary.Conv_DoubleToVector` 5000.0))) :`TraceChannel` "TraceTypeQuery5" :`DrawDebugType` "ForDuration"))
    (bind (_bblockinghit _binitialoverlap _time _distance _location _impactpoint _normal _impactnormal _physmat) (`GameplayStatics.BreakHitResult` _outhit))
    (`GameplayStatics.PlaySoundAtLocation` (select `EPhysicalSurface` (`PhysicalMaterial.SurfaceType` _physmat) :`SurfaceType1` "/Game/Sound/PhysicsSound/Bullet/concrete/concrete_impact_bullet_Cue.concrete_impact_bullet_Cue" :!type "SoundBase Object Reference") _location (struct) 1.0 1.0 0.0 null null null null)))

(fn `UserConstructionScript`)